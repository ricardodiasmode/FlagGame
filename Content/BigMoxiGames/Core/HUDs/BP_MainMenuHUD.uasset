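; BP_MainMenuHUD is the main menu HUD that switches between the main menu and find-match screens.
; On BeginPlay it opens WBP_MainMenu, and separate events create a fresh WBP_MainMenu or WBP_FindMatches widget on each navigation.
; A shared function removes the current widget from its parent, adds the new one to the viewport and stores it as CurrentWidget, so it shows one screen at a time.
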(event `self.ReceiveBeginPlay`
  (`self.GoToMainMenu`))

(event `GoToMainMenu`
  (bind _returnvalue (`|CreateWidget` "/Game/BigMoxiGames/UI/Menu/WBP_MainMenu.WBP_MainMenu_C"))
  (`self.TravelToWidgetAndRemovePrevious` _returnvalue))

(event `TravelToFindMatchWidget`
  (bind _returnvalue (`|CreateWidget` "/Game/BigMoxiGames/UI/Menu/WBP_FindMatches.WBP_FindMatches_C"))
  (`self.TravelToWidgetAndRemovePrevious` _returnvalue))

(fn `TravelToWidgetAndRemovePrevious`
  (params (InputPin :type "UserWidget Object Reference"))
  (bind _currentwidget (`self.CurrentWidget`)
    (:`then`
      (`Widget.RemoveFromParent` _currentwidget))
    (:`else`
      _))
  (`UserWidget.AddToViewport` InputPin 0)
  (set `self.CurrentWidget` InputPin))

(fn `UserConstructionScript`)