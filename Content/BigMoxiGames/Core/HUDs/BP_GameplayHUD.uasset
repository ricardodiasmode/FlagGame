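; BP_GameplayHUD is the in-match HUD that creates and manages the gameplay UMG widgets.
; On BeginPlay it adds WBP_MainScreen to the viewport.
; Weapon equip and dequip events swap or remove a single cached WBP_WeaponAmmo widget bound to the equipped weapon.
; When a team wins, an event shows WBP_WinCounter with the winning team and reset time.
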(event `self.ReceiveBeginPlay`
  (bind _returnvalue (`|CreateWidget` "/Game/BigMoxiGames/UI/Gameplay/Widget/WBP_MainScreen.WBP_MainScreen_C"))
  (`UserWidget.AddToViewport` _returnvalue 0))

(event `self.OnWeaponEquipped`
  (params (Weapon :type "Weapon Object Reference"))
  ;[1 1 1] Weapon equip/dequip
  (bind _weaponwidget (`self.WeaponWidget`)
    (:`then`
      (`Widget.RemoveFromParent` _weaponwidget))
    (:`else`
      _))
  (bind _returnvalue (`|CreateWidget` "/Game/BigMoxiGames/UI/Gameplay/Widget/WBP_WeaponAmmo.WBP_WeaponAmmo_C" null (struct :`AttributeName` "Ammo" :`Attribute` "/Script/BigMoxiGames.WeaponAttributeSet:Ammo" :`AttributeOwner` "/Script/CoreUObject.Class'/Script/BigMoxiGames.WeaponAttributeSet'") (struct :`AttributeName` "MaxAmmo" :`Attribute` "/Script/BigMoxiGames.WeaponAttributeSet:MaxAmmo" :`AttributeOwner` "/Script/CoreUObject.Class'/Script/BigMoxiGames.WeaponAttributeSet'") Weapon))
  (`UserWidget.AddToViewport` _returnvalue 0)
  (set `self.WeaponWidget` _returnvalue))

(event `self.OnWeaponDequipped`
  (params (Weapon :type "Weapon Object Reference"))
  ;[1 1 1] Weapon equip/dequip
  (bind _weaponwidget (`self.WeaponWidget`)
    (:`then`
      (`Widget.RemoveFromParent` _weaponwidget)
      (set `self.WeaponWidget` null))
    (:`else`)))

(event `self.StartCounterOnTeamWin`
  (params (PlayerTeam :type "EPlayerTeam Enum (by ref)" :default "Blue") (TimeToResetAfterMatchEnd :type "Float (single-precision)"))
  ;[1 1 1] Win Counter
  (bind _returnvalue (`|CreateWidget` "/Game/BigMoxiGames/UI/Gameplay/Widget/WBP_WinCounter.WBP_WinCounter_C" null TimeToResetAfterMatchEnd PlayerTeam))
  (`UserWidget.AddToViewport` _returnvalue 0))

(fn `UserConstructionScript`)